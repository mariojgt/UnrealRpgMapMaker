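; BP_WayPoint is a map waypoint actor that gets discovered when the player comes within range.
; Its DiscoverRange sphere, sized from DiscoverRadius in the construction script, passes the waypoint to DiscoverWaypoint on any overlapping actor's BPC_WorldMapRadar component.
; The OnDiscover event serves as the callback and only prints a debug string.
; A node that would destroy the sphere is unconnected, so overlaps can repeat the discovery call.
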(event OnComponentBeginOverlap(DiscoverRange)
  (params (OverlappedComponent :type Primitive%20Component%20Object%20Reference) (OtherActor :type Actor%20Object%20Reference) (OtherComp :type Primitive%20Component%20Object%20Reference) (OtherBodyIndex :type Integer) (bFromSweep :type Boolean) (SweepResult :type Hit%20Result%20Structure%20%28by%20ref%29))
  (bind _returnvalue (Actor|GetComponentbyClass OtherActor "/Game/MapSystem/Components/BPC_WorldMapRadar.BPC_WorldMapRadar_C"))
  ;[0.3235 1 0] On Player touch this element will trigger a event on the bpc component that will trigger discover and enable this waypoint in the map
  (Utilities|IsValid _returnvalue
    (:Is%20Valid
      (Default|DiscoverWaypoint _returnvalue self))))

(event Custom|OnDiscover
  ;[1 0.5203 0] This event execute run back here
  (Development|PrintString "way points discover"))

(event EventBeginPlay)

(event Collision|EventActorBeginOverlap
  (params (OtherActor :type Actor%20Object%20Reference)))

(event EventTick
  (params (DeltaSeconds :type Float%20%28single-precision%29)))

(fn ConstructionScript
  (Components|Sphere|SetSphereRadius (Variables|Default|GetDiscoverRange) (Variables|Settings|GetDiscoverRadius) false))