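; BP_BaseMapMarker is a base map marker actor that registers itself as a point of interest with overlapping map boundaries.
; With AutoStart on, it waits briefly after BeginPlay, then runs a server-to-multicast lookup through RemoveMarkerTrigger's overlaps, caching the boundary reference and adding itself to that boundary's list.
; If DestoryOnTouch is set, an overlapping actor's BPC_MasterGuidance component is told to remove the marker.
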(event OnComponentBeginOverlap(RemoveMarkerTrigger)
  (params (OverlappedComponent :type Primitive%20Component%20Object%20Reference) (OtherActor :type Actor%20Object%20Reference) (OtherComp :type Primitive%20Component%20Object%20Reference) (OtherBodyIndex :type Integer) (bFromSweep :type Boolean) (SweepResult :type Hit%20Result%20Structure%20%28by%20ref%29))
  (bind _returnvalue (Actor|GetComponentbyClass OtherActor "/Game/MasterGuidance/guidanceSystem/Components/BPC_MasterGuidance.BPC_MasterGuidance_C"))
  ;[1 1 1] On Actor enter check if have the valid map component if yes we can remove this marker
  (Utilities|IsValid _returnvalue
    (:Is%20Valid
      (if (Variables|Settings|GetbDestoryOnTouch)
        (Default|RemovePlayerMarker _returnvalue self)))))

(event Custom|GetBoundarieRef_server
  ;[1 1 1] Get the map boundarie overlap this actor
  (CallFunction|GetBoundarieRefMulticast))

(event Custom|GetBoundarieRef_multicast
  ;[1 1 1] Get the map boundarie overlap this actor
  (for _array_element (Collision|GetOverlappingActors (Variables|Default|GetRemoveMarkerTrigger) "/Game/MasterGuidance/guidanceSystem/Actors/MapBoundaries/BP_MapBoundaries.BP_MapBoundaries_C" :!class /Script/Engine.PrimitiveComponent)
    (Utilities|IsValid _array_element
      (:Is%20Valid
        (bind _boundariereturn (Class|BPIMapBoundaries|IReturnBoundarieRef(Message) _array_element))
        (bind _output_get (Variables|Default|SetMapBoundarieRef _boundariereturn))
        (Utilities|Array|AddUnique (Variables|/Game/MasterGuidance/guidanceSystem/Actors/MapBoundaries/BP_MapBoundaries.BP_MapBoundaries_C|GetMapPointsOfInterest _output_get) self)))))

(event EventBeginPlay
  ;[1 1 1] Wait 2 second to call the get boundaries on the server
  (if (Variables|Settings|GetAutoStart)
    (Utilities|FlowControl|Delay 0.3)
    (CallFunction|GetBoundarieRefServer)))

(event Collision|EventActorBeginOverlap
  (params (OtherActor :type Actor%20Object%20Reference)))

(event EventTick
  (params (DeltaSeconds :type Float%20%28single-precision%29)))

(fn ConstructionScript)