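; Fog-of-war area actor for the guidance system that reveals its map markers when discovered.
; On BeginPlay it multicasts a lookup that registers it with map boundaries overlapping its area sphere.
; A larger discover sphere, sized in the construction script, notifies an overlapping actor's MasterGuidance component once.
; On discovery, linked markers fetch their boundary references, the guidance system refreshes, and the actor destroys itself.
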(event OnComponentBeginOverlap(DiscoverSphere)
  (params (OverlappedComponent :type Primitive%20Component%20Object%20Reference) (OtherActor :type Actor%20Object%20Reference) (OtherComp :type Primitive%20Component%20Object%20Reference) (OtherBodyIndex :type Integer) (bFromSweep :type Boolean) (SweepResult :type Hit%20Result%20Structure%20%28by%20ref%29))
  (bind _returnvalue (Actor|GetComponentbyClass OtherActor "/Game/MasterGuidance/guidanceSystem/Components/BPC_MasterGuidance.BPC_MasterGuidance_C"))
  ;[0 1 0.08199] On the object that have the component touch this will trigget the undiscover the area
  (Utilities|IsValid _returnvalue
    (:Is%20Valid
      (Utilities|FlowControl|DoOnce false
        (:Completed
          (Default|OnDiscoverArea _returnvalue self))))))

(event Custom|OnDiscovered
  (params (MasterGuidance :type BPC%20Master%20Guidance%20Object%20Reference))
  ;[1 0.08006 0] This is trigger after the bpc register the event
  (for _array_element (Variables|Settings|GetMarkerToDiscover)
    (Default|GetBoundarieRefServer _array_element))
  (Default|APIRefreshGuidanceSystem MasterGuidance)
  (Actor|DestroyActor))

(event Custom|API_GetBoundarie_Server
  ;[1 1 1] Get the boundires
  (CallFunction|APIGetBoundarieMulticast))

(event Custom|API_GetBoundarie_Multicast
  ;[1 1 1] Get the boundires
  (for _array_element (Collision|GetOverlappingActors (Variables|Default|GetAreaShepere) "/Game/MasterGuidance/guidanceSystem/Actors/MapBoundaries/BP_MapBoundaries.BP_MapBoundaries_C" :!class /Script/Engine.PrimitiveComponent)
    (Utilities|IsValid _array_element
      (:Is%20Valid
        (bind _boundariereturn (Class|BPIMapBoundaries|IReturnBoundarieRef(Message) _array_element))
        (bind _output_get (Variables|Default|SetMapBoundarieRef _boundariereturn))
        (Utilities|Array|AddUnique (Variables|/Game/MasterGuidance/guidanceSystem/Actors/MapBoundaries/BP_MapBoundaries.BP_MapBoundaries_C|GetBoundariesFogOfWar _output_get) self)))))

(event EventBeginPlay
  ;[1 1 1] Get the boundires
  (CallFunction|APIGetBoundarieServer))

(fn ConstructionScript
  (bind _arearadius (Variables|Settings|GetAreaRadius))
  (Components|Sphere|SetSphereRadius (Variables|Default|GetAreaShepere) _arearadius false)
  (Components|Sphere|SetSphereRadius (Variables|Default|GetDiscoverSphere) (+ _arearadius (Variables|Settings|GetAddicionalDiscoverRadius)) false))