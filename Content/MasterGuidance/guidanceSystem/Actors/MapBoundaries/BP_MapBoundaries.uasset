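; BP_MapBoundaries is a map area actor for the MasterGuidance system, defined by two corner actors and holding map points of interest.
; Its construction script centers it between the corners in XY and can auto-size its trigger as a cube from their Y distance.
; Overlapping actors with BPC_MasterGuidance receive it as their boundary update.
; A server-to-multicast event pair removes points of interest, and an interface function returns the actor itself.
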(event OnComponentBeginOverlap(UpdateMapBoundarieTrigger)
  (params (OverlappedComponent :type Primitive%20Component%20Object%20Reference) (OtherActor :type Actor%20Object%20Reference) (OtherComp :type Primitive%20Component%20Object%20Reference) (OtherBodyIndex :type Integer) (bFromSweep :type Boolean) (SweepResult :type Hit%20Result%20Structure%20%28by%20ref%29))
  (bind _returnvalue (Actor|GetComponentbyClass OtherActor "/Game/MasterGuidance/guidanceSystem/Components/BPC_MasterGuidance.BPC_MasterGuidance_C"))
  ;[0.4364 1 0] Once the player enter the mao boundaries we goin to call the event to update the current player boundarie
  (Utilities|IsValid _returnvalue
    (:Is%20Valid
      (Default|OnBoundarieUpdate _returnvalue self))))

(event Custom|RemoveItem_server
  (params (Item :type WBP%20Base%20Map%20Marker%20Object%20Reference%20%28by%20ref%29))
  ;[1 1 1] Remove map points of interest
  (CallFunction|RemoveItemMulticast Item))

(event Custom|RemoveItem_multicast
  (params (Item :type WBP%20Base%20Map%20Marker%20Object%20Reference%20%28by%20ref%29))
  ;[1 1 1] Remove map points of interest
  (Utilities|Array|RemoveItem (Variables|MapBoundariesSettings|GetMapPointsOfInterest) Item))

(event EventBeginPlay)

(event Collision|EventActorBeginOverlap
  (params (OtherActor :type Actor%20Object%20Reference)))

(event EventTick
  (params (DeltaSeconds :type Float%20%28single-precision%29)))

(fn ConstructionScript
  (bind _returnvalue (Math|Float|MakeLiteralFloat 2.0))
  (bind _returnvalue_2 (CallFunction|GetMapWidth))
  (bind _lowerleftcorner (Variables|Default|GetLowerLeftCorner))
  (bind _upperrightcorner (Variables|Default|GetUpperRightCorner))
  (bind _returnvalue_3 (Transformation|GetActorLocation _lowerleftcorner))
  (bind _returnvalue_4 (Transformation|GetActorLocation _upperrightcorner))
  (bind _returnvalue_5 (- _returnvalue_3 _returnvalue_4))
  (bind _returnvalue_6 (/ _returnvalue_5 _returnvalue))
  (bind _returnvalue_7 (+ _returnvalue_4 _returnvalue_6))
  (bind (_x _y) (Math|Vector|BreakVector _returnvalue_7))
  ;[1 1 1] Make sure the upper left conner and lower right conner is valid
  (if (and (Utilities|IsValid (Variables|Default|GetUpperRightCorner)) (Utilities|IsValid (Variables|Default|GetLowerLeftCorner)))
    (Transformation|SetActorLocation (Math|Vector|MakeVector _x _y (.z (Transformation|GetActorLocation))) false true)
    ;[1 1 1] Check if this boundarie is ogin to use auto trigger resize
    (if (Variables|MapBoundariesSettings|GetAutoResizeTriggerToMap)
      (Components|Box|SetBoxExtent (Variables|Default|GetUpdateMapBoundarieTrigger) (Math|Vector|MakeVector _returnvalue_2 _returnvalue_2 _returnvalue_2) true))
    (else
      (Development|PrintString "Please Setup the upper left corner and Lower right corner"))))

(fn GetMapWidth
  (return (* (/ (Math|Float|Absolute(Float) (- (.Y (Math|Vector|BreakVector (Transformation|GetActorLocation (Variables|Default|GetLowerLeftCorner)))) (.Y (Math|Vector|BreakVector (Transformation|GetActorLocation (Variables|Default|GetUpperRightCorner)))))) 2.0) (Variables|MapBoundariesSettings|GetTriggerOffsetMultiplier))))

(fn IReturnBoundarieRef
  (return self))